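; Showcase actor for a finite state machine component, running separate movement and rotation state machines started once on the server.
; The movement machine alternates OffsetX and OffsetY states, whose timelines flip between forward and reverse to move the actor around its start location.
; The rotation machine adds yaw each tick, using delays in the Rotate state's enter and exit events to alternate spinning and pausing.
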(event Custom|StartStateMachine
  (Networking|SwitchHasAuthority
    (:Authority
      (Utilities|FlowControl|DoOnce false
        (:Completed
          (Class|FiniteStateMachineComponent|SetState (Variables|Default|GetFiniteStateMachine) "OffsetX")
          (Class|FiniteStateMachineComponent|SetState (Variables|Default|GetRotateStateMachine) "Rotate"))))))

(event EventBeginPlay
  (Variables|Default|SetStartLocation (Transformation|GetActorLocation))
  (Variables|Default|SetStartRotation (Transformation|GetActorRotation)))

(fn ConstructionScript)